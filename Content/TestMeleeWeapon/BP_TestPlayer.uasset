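; BP_TestPlayer is a test player character that starts play with a melee weapon in hand and a link to its inventory UI.
; BeginPlay spawns BP_BaseWeapon at the mesh's WeaponSocket, sets itself as owner and snaps the weapon to that socket.
; It then casts the InventoryComponent's widget to WBP_Inventory and caches it.
; Tick does nothing, the overlap event is disabled, and an attack montage call is left unwired.
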(event `self.ReceiveBeginPlay`
  (bind _mesh (`self.Mesh`))
  (`parent.ReceiveBeginPlay`)
  (bind _returnvalue (`|SpawnActorFromClass` "/Game/Weapon/BP_BaseWeapon.BP_BaseWeapon_C" (`KismetMathLibrary.MakeTransform` (`SceneComponent.GetSocketLocation` _mesh "WeaponSocket") (`SceneComponent.GetSocketRotation` _mesh "WeaponSocket")) "AlwaysSpawn" "MultiplyWithRoot" null null))
  (bind _output_get (set `self.MeleeWeaponRef` _returnvalue))
  (`self.SetOwner` _output_get self)
  (`self.K2_AttachToComponent` _output_get (`self.Mesh`) "WeaponSocket" "SnapToTarget" "SnapToTarget" "SnapToTarget" true)
  (bind _aswbp_inventory (cast `/Game/Inventory/Widgets/WBP_Inventory` (`InventoryComponent.InventoryWidget` (`self.InventoryComponent`))))
  (set `self.WBP_InventoryWidget` _aswbp_inventory))

(event `self.ReceiveTick`
  (params (DeltaSeconds :type "Float (single-precision)")))

(event `Key|LeftMouseButton`
  (params (Key :type "Key Structure")))

(fn `UserConstructionScript`
  (`parent.UserConstructionScript`))