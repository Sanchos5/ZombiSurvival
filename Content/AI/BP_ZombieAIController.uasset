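; AI controller for zombies that detects the player and handles losing track of them.
; It runs BT_Zombie and caches the controlled BP_Zombie on BeginPlay.
; Player perception updates set or clear the TargetActor blackboard key.
; When the player is lost, the controller itself issues a move to the last stimulus location, then after a short delay returns the zombie to its start point, outside the behavior tree.
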(event `self.ReceiveBeginPlay`
  (`self.RunBehaviorTree` "/Game/AI/BT_Zombie.BT_Zombie")
  (bind _asbp_zombie (cast `/Game/Characters/Enemy/BP_Zombie` (`self.K2_GetPawn`)))
  (set `self.Zombie Ref` _asbp_zombie))

(event `self.AIPerception.OnPerceptionUpdated`
  (params (UpdatedActors :type "Array of Actor Object Reference (by ref)")))

(event `self.AIPerception.OnTargetPerceptionUpdated`
  (params (Actor :type "Actor Object Reference") (Stimulus :type "AIStimulus Structure"))
  (bind (_age _expirationage _strength _stimuluslocation _receiverlocation _tag _bsuccessfullysensed) (break `AIStimulus` Stimulus))
  (bind _blackboard (`self.Blackboard`))
  (if (== Actor (`GameplayStatics.GetPlayerPawn` 0))
    (if _bsuccessfullysensed
      (`BlackboardComponent.SetValueAsObject` _blackboard "TargetActor" Actor)
      (else
        (`BlackboardComponent.ClearValue` _blackboard "TargetActor")
        (`AITask_MoveTo.AIMoveTo` null _stimuluslocation null
          (:`OnMoveFinished`
            (`KismetSystemLibrary.Delay` 5.0)
            (bind _zombie_ref (`self.Zombie Ref`)
              (:`then`
                (`self.MoveToLocation` (`/Game/Characters/Enemy/BP_Zombie.Start Point Location` _zombie_ref) -1.0 true true false true null))
              (:`else`))))))))

(event `self.AIPerception.OnTargetPerceptionInfoUpdated`
  (params (UpdateInfo :type "ActorPerceptionUpdateInfo Structure (by ref)")))

(fn `UserConstructionScript`)