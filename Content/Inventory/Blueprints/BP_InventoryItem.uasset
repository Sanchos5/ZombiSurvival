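; BP_InventoryItem is a pickup actor in the world that the player collects into their inventory on interaction.
; The construction script looks up the item's ID in DT_ItemInfo and sets the static mesh from that row.
; Interact passes the item to the BP_TestPlayer's InventoryComponent; on success it destroys itself and refreshes the UI for its item type (melee, range or eatables) plus the main inventory UI.
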(event `InteractionInterface.Interact`
  (params (InstigatorPawn :type "Pawn Object Reference"))
  (bind _item (`self.Item`))
  (bind _asbp_test_player (cast `/Game/TestMeleeWeapon/BP_TestPlayer` (`GameplayStatics.GetPlayerCharacter` 0)))
  (bind _inventorycomponent (`SurvivalPlayer.InventoryComponent` _asbp_test_player))
  (`/Engine/EditorBlueprintResources/StandardMacros.IsValid` _inventorycomponent
    (:`Is Valid`
      (bind _returnvalue (`InventoryComponent.AddToInventory` _inventorycomponent _item))
      (if _returnvalue
        (`self.K2_DestroyActor`)
        (switch `EItemType` (`.ItemType` (break `Slot` _item))
          (:`EI_MeleeWeapon`
            (`InventoryComponent.UpdateMeleeWeaponUI` _inventorycomponent))
          (:`EI_RangeWeapon`
            (`InventoryComponent.UpdateRangeWeaponUI` _inventorycomponent))
          (:`EI_Eatables`
            (`InventoryComponent.UpdateEatablesUI` _inventorycomponent)))
        (`InventoryComponent.UpdateMainInventoryUI` _inventorycomponent)))))

(fn `UserConstructionScript`
  (bind _returnvalue (`|GetDataTableRow` "/Game/Inventory/DataTables/DT_ItemInfo.DT_ItemInfo" (`.RowName` (break `DataTableRowHandle` (`.ItemID` (break `Slot` (`self.Item`))))))
    (:`then`
      (`StaticMeshComponent.SetStaticMesh` (`self.StaticMesh`) (`.Mesh` (break `ItemInfo` _returnvalue))))))