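; Player character Blueprint that handles weapon swapping, firing and reloading, and keeps the HUD in sync.
; Swap events call the parent logic, then update the weapon and ammo bars and link the matching animation class layer for axe, pistol or shotgun.
; Attack and reload forward to the ranged weapon, with a reload montage for the shotgun only.
; It also clamps camera pitch every tick and increments hunger on the F key.
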(event `self.ReceiveBeginPlay`
  (bind _asbp_hud (cast `/Game/UI/BP_HUD` (`PlayerController.GetHUD` (`GameplayStatics.GetPlayerController` 0))))
  (set `self.Player Interface` (`/Game/UI/BP_HUD.PlayerInterface` _asbp_hud))
  (`SkeletalMeshComponent.LinkAnimClassLayers` (`self.Mesh`) "/Game/Animations/Player/Locomotion/Unarmed/ABP_Unarmed.ABP_Unarmed_C"))

(event `self.ReceiveTick`
  (params (DeltaSeconds :type "Float (single-precision)"))
  (bind _returnvalue (`GameplayStatics.GetPlayerCameraManager` 0))
  (set `PlayerCameraManager.ViewPitchMin` -60.0 _returnvalue)
  (set `PlayerCameraManager.ViewPitchMax` 60.0 _returnvalue))

(event `Key|F`
  (params (Key :type "Key Structure"))
  (:`Pressed`
    (`PlayerStatsComponent.IncrementHunger` (`self.PlayerStats`) 10.0)))

(event `self.Input_SwapToAxe`
  (params (InputActionValue :type "InputActionValue Structure (by ref)"))
  (bind _player_interface (`self.Player Interface`))
  ;[1 1 1] Выбран топор
  (`parent.Input_SwapToAxe` InputActionValue)
  (if (`|EnumEquality` (`self.ActiveWeapon`) "AXE")
    (`Widget.SetVisibility` (`/Game/UI/InterfaceGame/WBP_InterfacePlayer.WBP_PatronBar` _player_interface) "Hidden")
    (`/Game/UI/WidgetPlayer/WeaponBar/WBP_WeaponBar.SelectAxe` (`/Game/UI/InterfaceGame/WBP_InterfacePlayer.WBP_WeaponBar` _player_interface))
    (`SkeletalMeshComponent.LinkAnimClassLayers` (`self.Mesh`) "/Game/Animations/Player/Locomotion/Axe/ABP_Axe.ABP_Axe_C")))

(event `self.Input_SwapToPistol`
  (params (InputActionValue :type "InputActionValue Structure (by ref)"))
  (bind _player_interface (`self.Player Interface`))
  (bind _wbp_patronbar (`/Game/UI/InterfaceGame/WBP_InterfacePlayer.WBP_PatronBar` _player_interface))
  ;[1 1 1] Выбран наган
  (`parent.Input_SwapToPistol` InputActionValue)
  (if (`|EnumEquality` (`self.ActiveWeapon`) "PISTOL")
    (`Widget.SetVisibility` _wbp_patronbar "Visible")
    (`/Game/UI/WidgetPlayer/PatronBar/WBP_PatronBar.InitializePatron` _wbp_patronbar)
    (`/Game/UI/WidgetPlayer/PatronBar/WBP_PatronBar.PatronsInInventory` _wbp_patronbar)
    (`/Game/UI/WidgetPlayer/WeaponBar/WBP_WeaponBar.SelectPistol` (`/Game/UI/InterfaceGame/WBP_InterfacePlayer.WBP_WeaponBar` _player_interface))
    (`SkeletalMeshComponent.LinkAnimClassLayers` (`self.Mesh`) "/Game/Animations/Player/Locomotion/Pistol/ABP_Pistol.ABP_Pistol_C")))

(event `self.Input_SwapToShotgun`
  (params (InputActionValue :type "InputActionValue Structure (by ref)"))
  (bind _player_interface (`self.Player Interface`))
  (bind _wbp_patronbar (`/Game/UI/InterfaceGame/WBP_InterfacePlayer.WBP_PatronBar` _player_interface))
  ;[1 1 1] Выбран двухстволка
  (`parent.Input_SwapToShotgun` InputActionValue)
  (if (`|EnumEquality` (`self.ActiveWeapon`) "SHOTGUN")
    (`Widget.SetVisibility` _wbp_patronbar "Visible")
    (`/Game/UI/WidgetPlayer/PatronBar/WBP_PatronBar.InitializePatron` _wbp_patronbar)
    (`/Game/UI/WidgetPlayer/PatronBar/WBP_PatronBar.PatronsInInventory` _wbp_patronbar)
    (`/Game/UI/WidgetPlayer/WeaponBar/WBP_WeaponBar.SelectShotgun` (`/Game/UI/InterfaceGame/WBP_InterfacePlayer.WBP_WeaponBar` _player_interface))
    (`SkeletalMeshComponent.LinkAnimClassLayers` (`self.Mesh`) "/Game/Animations/Player/Locomotion/Shotgun/ABP_Shotgun.ABP_Shotgun_C")))

(event `EnhancedInput|/Game/Characters/Input/Actions/IA_Attack`
  (params (ActionValue :type Boolean) (ElapsedSeconds :type "Float (double-precision)") (TriggeredSeconds :type "Float (double-precision)") (InputAction :type "InputAction Object Reference" :default "/Game/Characters/Input/Actions/IA_Attack.IA_Attack"))
  ;[1 1 1] Стрельба
  (:`Started`
    (bind _rangeweaponref (`self.RangeWeaponref`)
      (:`then`
        (bind _asbp_abstract_gun (cast `/Game/Weapon/WeaponToFight/BP_abstract_gun` _rangeweaponref))
        (`/Game/Weapon/WeaponToFight/BP_abstract_gun.Shoot` _asbp_abstract_gun))
      (:`else`))))

(event `InputAction|upr_R`
  (params (Key :type "Key Structure"))
  ;[1 1 1] Перезарядка
  (:`Pressed`
    (bind _rangeweaponref (`self.RangeWeaponref`)
      (:`then`
        (bind _asbp_abstract_gun (cast `/Game/Weapon/WeaponToFight/BP_abstract_gun` _rangeweaponref))
        (`/Game/Weapon/WeaponToFight/BP_abstract_gun.Reload` _asbp_abstract_gun)
        (if (`|EnumEquality` (`self.ActiveWeapon`) "SHOTGUN")
          (`self.PlayAnimMontage` "/Game/Animations/Player/AM_Reload.AM_Reload")))
      (:`else`))))

(fn `UserConstructionScript`)