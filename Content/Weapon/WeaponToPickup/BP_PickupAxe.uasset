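; BP_PickupAxe is an interactable axe pickup that gives the player the axe weapon.
; On interact, it updates the player's weapon bar UI and calls the player's axe pickup event.
; At BeginPlay it binds to player 0's pickup-axe dispatcher, destroying itself when that fires.
; It also supplies its interaction prompt text.
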(event `InteractionInterface.Interact`
  (params (InstigatorPawn :type "Pawn Object Reference"))
  (bind _asbp_player (cast `/Game/Characters/Player/BP_Player` InstigatorPawn))
  (`/Game/UI/WidgetPlayer/WeaponBar/WBP_WeaponBar.GetAxe` (`/Game/UI/InterfaceGame/WBP_InterfacePlayer.WBP_WeaponBar` (`/Game/Characters/Player/BP_Player.Player Interface` _asbp_player)))
  (`/Game/Characters/Player/BP_Player.Event_PickUpAxe` _asbp_player))

(event `self.ReceiveBeginPlay`
  (bind _asbp_player (cast `/Game/Characters/Player/BP_Player` (`GameplayStatics.GetPlayerCharacter` 0)))
  (add `/Game/Characters/Player/BP_Player.PickupAxe` _asbp_player (delegate `PickupAxe_Event`)))

(event `PickupAxe_Event`
  (`self.K2_DestroyActor`))

(fn `GetInteractText`
  (returns (ReturnValue :type Text))
  (return (`self.InteractionText`)))

(fn `UserConstructionScript`
  (`parent.UserConstructionScript`))