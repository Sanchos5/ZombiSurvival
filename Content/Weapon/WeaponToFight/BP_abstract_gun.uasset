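; Base gun Blueprint for the player's pistol and shotgun, handling firing, ammo and reloading against zombies.
; Shoot spends magazine ammo and fires randomly spread line traces along control rotation, looping for shotgun pellets, to damage and push zombies.
; An empty magazine triggers player reload input, with a shotgun-specific animation via a child cast.
; Reload moves matching inventory ammo into the magazine, drawing on a second stack if needed, and updates the HUD.
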(event `self.ReceiveBeginPlay`
  (bind _asbp_hud (cast `/Game/UI/BP_HUD` (`PlayerController.GetHUD` (`GameplayStatics.GetPlayerController` 0))))
  (set `self.Player Interface` (`/Game/UI/BP_HUD.PlayerInterface` _asbp_hud)))

(event `self.ReceiveTick`
  (params (DeltaSeconds :type "Float (single-precision)")))

(event `Event_shot`
  (`ActorComponent.Activate` (`self.ParticleSystem`) true))

(event `Shoot`
  ;[1 1 1] Стрелять
  (if (`AnimInstance.Montage_IsPlaying` (`SkeletalMeshComponent.GetAnimInstance` (`Character.Mesh` (`GameplayStatics.GetPlayerCharacter` 0))) "/Game/Animations/Player/AM_Reload.AM_Reload")
    _
    (elif (> (`self.DispenserMagazine`) 0)
      (message `/Game/Blueprints/Interface/BPI_Patrons.ConsumePatron` (`/Game/UI/InterfaceGame/WBP_InterfacePlayer.WBP_PatronBar` (`self.Player Interface`)))
      (set `self.DispenserMagazine` (- (`self.DispenserMagazine`) 1))
      (if (== (`self.PatronName`) "PistolPatron")
        (`GameplayStatics.PlaySound2D` "/Game/Sounds/Weapons_Sounds/WAV_Pistol_Shot02.WAV_Pistol_Shot02" 1.0 1.0 0.0 null null)
        (`self.ShotLineTrace` (`self.Damage`) :!label _label)
        (else
          (`GameplayStatics.PlaySound2D` "/Game/Sounds/Weapons_Sounds/WAV_Shotgun_Shot.WAV_Shotgun_Shot" 1.0 1.0 0.0 null null)
          (`self.ShotLineTrace` (`self.Damage`))
          (`self.Event_shot`)
          (for _ (range 1 (+ (`self.Number of shotgun bullets`) 1))
            (goto _label))))
      (else
        (`GameplayStatics.PlaySound2D` "/Game/Sounds/Weapons_Sounds/WAV_Weapon_Empty.WAV_Weapon_Empty" 1.0 1.0 0.0 null null)
        (bind _asbp_player (cast `/Game/Characters/Player/BP_Player` (`GameplayStatics.GetPlayerCharacter` 0)))
        (`SurvivalPlayer.Input_Reloading` _asbp_player (`EnhancedInputLibrary.MakeInputActionValueOfType` 0.0 0.0 0.0 "Boolean"))
        (bind _asbp_shotgun (cast `/Game/Weapon/WeaponToFight/BP_shotgun` self))
        (if (and (> (`BaseRangeWeapon.PatronsInInventory` _asbp_shotgun) 0) (!= (`BaseRangeWeapon.DispenserMagazine` _asbp_shotgun) (`BaseRangeWeapon.MaxDispenserMagazine` _asbp_shotgun)))
          (`/Game/Weapon/WeaponToFight/BP_shotgun.Play Reload Anim` _asbp_shotgun))))))

(event `Reload`
  ;[1 1 1] Перезарядка
  (`self.ReloadDispenserMagazine`)
  (if (< (`self.DispenserMagazine`) (`self.MaxDispenserMagazine`))
    (`self.ReloadDispenserMagazine`))
  (message `/Game/Blueprints/Interface/BPI_Patrons.ReloadPatron` (`/Game/UI/InterfaceGame/WBP_InterfacePlayer.WBP_PatronBar` (`self.Player Interface`)) (`self.DispenserMagazine`)))

(fn `DecrementPatrons`
  (params (Array :type "Array of Slot Structure") (Index :type Integer) (IncrementInt :type Integer))
  (bind _index (`local.Index`))
  (bind (_itemid _quantity _itemtype) (break `Slot` (`|GetArrayItem` Array Index)))
  (bind _returnvalue (- _quantity IncrementInt))
  (if (> _returnvalue 0)
    (`KismetArrayLibrary.Array_Set` Array _index (make `Slot` _itemid _returnvalue _itemtype))
    (else
      (`KismetArrayLibrary.Array_Set` Array _index (make `Slot` (struct)))))
  (`InventoryComponent.UpdateAllInventoryUI` (`self.GetComponentByClass` (`GameplayStatics.GetPlayerCharacter` 0) "/Script/ZombiSurvival.InventoryComponent")))

(fn `ReloadDispenserMagazine`
  (for (_array_element _array_index) (`.MainInventory` (break `AllItem` (`InventoryComponent.AllItems` (`self.GetComponentByClass` (`GameplayStatics.GetPlayerCharacter` 0) "/Script/ZombiSurvival.InventoryComponent"))))
    (bind ((`ItemID` _itemid) (`Quantity` _quantity)) (break `Slot` _array_element))
    (if (and (== (`.RowName` (break `DataTableRowHandle` _itemid)) (`self.PatronName`)) (> _quantity 0))
      (for _ (range 1 (+ _quantity 1))
        (if (>= (`self.DispenserMagazine`) (`self.MaxDispenserMagazine`))
          (break)
          (else
            (`/Engine/EditorBlueprintResources/StandardMacros.IncrementInt` (`self.DispenserMagazine`)
              (:`  `
                (`/Engine/EditorBlueprintResources/StandardMacros.IncrementInt` (`self.Decrement Patrons Int`)))))))
      (`self.DecrementPatrons` (`.MainInventory` (break `AllItem` (`InventoryComponent.AllItems` (`self.GetComponentByClass` (`GameplayStatics.GetPlayerCharacter` 0) "/Script/ZombiSurvival.InventoryComponent")))) _array_index (`self.Decrement Patrons Int`))
      (set `self.Decrement Patrons Int` 0)
      (break))))

(fn `ShotLineTrace`
  (params (damage :type "Float (double-precision)"))
  (bind _returnvalue (`GameplayStatics.GetPlayerCharacter` 0))
  (bind _accuracy (`self.Accuracy`))
  (bind _accuracy_2 (`self.Accuracy`))
  (bind _accuracy_3 (`self.Accuracy`))
  (bind _returnvalue_2 (+ (`self.K2_GetActorLocation` _returnvalue) (0.0 0.0 65.0)))
  (bind _returnvalue_3 (+ (* (`KismetMathLibrary.Conv_RotatorToVector` (`Pawn.GetControlRotation` _returnvalue)) 25000.0) (`KismetMathLibrary.MakeVector` (`KismetMathLibrary.RandomFloatInRange` (* _accuracy_2 -1.0) _accuracy_2) (`KismetMathLibrary.RandomFloatInRange` (* _accuracy_3 -1.0) _accuracy_3) (`KismetMathLibrary.RandomFloatInRange` (* _accuracy -1.0) _accuracy))))
  (bind _outhit (`KismetSystemLibrary.LineTraceSingleForObjects` _returnvalue_2 (+ _returnvalue_2 _returnvalue_3) (`|MakeArray` "ObjectTypeQuery3" :!type "EObjectTypeQuery Enum") true (`|MakeArray` (`GameplayStatics.GetPlayerCharacter` 0) :!type "Actor Object Reference")))
  (bind (_bblockinghit _binitialoverlap _time _distance _location _impactpoint _normal _impactnormal _physmat _hitactor) (`GameplayStatics.BreakHitResult` _outhit))
  (bind _asbp_zombie (cast `/Game/Characters/Enemy/BP_Zombie` _hitactor))
  (`GameplayStatics.ApplyDamage` _asbp_zombie damage)
  (`PrimitiveComponent.AddImpulseAtLocation` (`Character.Mesh` _asbp_zombie) (* _returnvalue_3 (`self.Impulse`)) _impactpoint "None"))

(fn `UserConstructionScript`)