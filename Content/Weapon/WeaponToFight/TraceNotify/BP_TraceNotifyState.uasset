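; Anim notify state that opens and closes the melee weapon's trace window during the player's animations.
; On begin and end it casts the mesh owner to BP_Player, gets the TraceComponent on its MeleeWeaponRef and, if valid, sets WeaponActive true and false respectively.
; Owners that are not BP_Player are ignored.
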(fn `Received_NotifyBegin`
  (params (MeshComp :type "SkeletalMeshComponent Object Reference") (Animation :type "AnimSequenceBase Object Reference") (TotalDuration :type "Float (single-precision)") (EventReference :type "AnimNotifyEventReference Structure (by ref)"))
  (returns (ReturnValue :type Boolean))
  (bind _asbp_player (cast `/Game/Characters/Player/BP_Player` (`ActorComponent.GetOwner` MeshComp)))
  (bind _returnvalue (`Actor.GetComponentByClass` (`/Game/Characters/Player/BP_Player.MeleeWeaponRef` _asbp_player) "/Script/ZombiSurvival.TraceComponent"))
  (`/Engine/EditorBlueprintResources/StandardMacros.IsValid` _returnvalue
    (:`Is Valid`
      (bind _output_get (set `TraceComponent.WeaponActive` true _returnvalue))
      (return _output_get))))

(fn `Received_NotifyEnd`
  (params (MeshComp :type "SkeletalMeshComponent Object Reference") (Animation :type "AnimSequenceBase Object Reference") (EventReference :type "AnimNotifyEventReference Structure (by ref)"))
  (returns (ReturnValue :type Boolean))
  (bind _asbp_player (cast `/Game/Characters/Player/BP_Player` (`ActorComponent.GetOwner` MeshComp)))
  (bind _returnvalue (`Actor.GetComponentByClass` (`/Game/Characters/Player/BP_Player.MeleeWeaponRef` _asbp_player) "/Script/ZombiSurvival.TraceComponent"))
  (`/Engine/EditorBlueprintResources/StandardMacros.IsValid` _returnvalue
    (:`Is Valid`
      (bind _output_get (set `TraceComponent.WeaponActive` false _returnvalue))
      (return _output_get))))