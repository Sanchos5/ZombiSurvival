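; Anim notify state that opens and closes the weapon trace window during BP_Zombie animations.
; On begin it casts the mesh owner to BP_Zombie and sets WeaponActive on the TraceComponent of the left or right weapon, chosen by the LeftAnimation flag.
; On end it clears the same flag, so the weapon is only active for the span of the notify.
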(fn `Received_NotifyBegin`
  (params (MeshComp :type "SkeletalMeshComponent Object Reference") (Animation :type "AnimSequenceBase Object Reference") (TotalDuration :type "Float (single-precision)") (EventReference :type "AnimNotifyEventReference Structure (by ref)"))
  (returns (ReturnValue :type Boolean))
  (bind _asbp_zombie (cast `/Game/Characters/Enemy/BP_Zombie` (`ActorComponent.GetOwner` MeshComp)))
  (if (`self.LeftAnimation`)
    (bind _returnvalue (`Actor.GetComponentByClass` (`/Game/Characters/Enemy/BP_Zombie.LeftWeapon` _asbp_zombie) "/Script/ZombiSurvival.TraceComponent"))
    (`/Engine/EditorBlueprintResources/StandardMacros.IsValid` _returnvalue
      (:`Is Valid`
        (bind _output_get (set `TraceComponent.WeaponActive` true _returnvalue))
        (return _output_get)))
    (else
      (bind _returnvalue_2 (`Actor.GetComponentByClass` (`/Game/Characters/Enemy/BP_Zombie.RightWeapon` _asbp_zombie) "/Script/ZombiSurvival.TraceComponent"))
      (`/Engine/EditorBlueprintResources/StandardMacros.IsValid` _returnvalue_2
        (:`Is Valid`
          (bind _output_get_2 (set `TraceComponent.WeaponActive` true _returnvalue_2))
          (return _output_get_2))))))

(fn `Received_NotifyEnd`
  (params (MeshComp :type "SkeletalMeshComponent Object Reference") (Animation :type "AnimSequenceBase Object Reference") (EventReference :type "AnimNotifyEventReference Structure (by ref)"))
  (returns (ReturnValue :type Boolean))
  (bind _asbp_zombie (cast `/Game/Characters/Enemy/BP_Zombie` (`ActorComponent.GetOwner` MeshComp)))
  (if (`self.LeftAnimation`)
    (bind _returnvalue (`Actor.GetComponentByClass` (`/Game/Characters/Enemy/BP_Zombie.LeftWeapon` _asbp_zombie) "/Script/ZombiSurvival.TraceComponent"))
    (`/Engine/EditorBlueprintResources/StandardMacros.IsValid` _returnvalue
      (:`Is Valid`
        (bind _output_get (set `TraceComponent.WeaponActive` false _returnvalue))
        (return _output_get)))
    (else
      (bind _returnvalue_2 (`Actor.GetComponentByClass` (`/Game/Characters/Enemy/BP_Zombie.RightWeapon` _asbp_zombie) "/Script/ZombiSurvival.TraceComponent"))
      (`/Engine/EditorBlueprintResources/StandardMacros.IsValid` _returnvalue_2
        (:`Is Valid`
          (bind _output_get_2 (set `TraceComponent.WeaponActive` false _returnvalue_2))
          (return _output_get_2))))))