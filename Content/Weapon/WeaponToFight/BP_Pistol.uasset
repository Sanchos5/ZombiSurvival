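; Pistol weapon Blueprint for a Nagan with cartridge-by-cartridge reloading.
; Custom events play weapon mesh animations for reload start, adding a round, reload end and round removal.
; The reload function finds matching ammo in the owning player's inventory, loads one round if space remains, and updates the patron bar widget.
; It searches the owner's inventory but decrements player character 0's, assuming both are the same.
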(event `StartNaganReload`
  (`SkeletalMeshComponent.PlayAnimation` (`self.WeaponMesh`) (`self.StartNaganReloadAnim`) false))

(event `PlayDeletePatron`
  (`SkeletalMeshComponent.PlayAnimation` (`self.WeaponMesh`) (`self.DeletePatronAnim`) false))

(event `EndNaganReload`
  (`SkeletalMeshComponent.PlayAnimation` (`self.WeaponMesh`) (`self.EndNaganReloadAnim`) false))

(event `AddPatron`
  (`SkeletalMeshComponent.PlayAnimation` (`self.WeaponMesh`) (`self.AddPatronAnim`) false))

(fn `ReloadDispenserMagazine_Nagan`
  (bind _returnvalue (`self.GetOwner`))
  (`/Engine/EditorBlueprintResources/StandardMacros.IsValid` _returnvalue
    (:`Is Valid`
      (bind _asbp_player_camera (cast `/Game/Blueprints/BP_Player_Camera` _returnvalue))
      (for (_array_element _array_index) (`.MainInventory` (break `AllItem` (`InventoryComponent.AllItems` (`SurvivalPlayer.InventoryComponent` _asbp_player_camera))))
        (bind ((`ItemID` _itemid) (`Quantity` _quantity)) (break `Slot` _array_element))
        (if (and (== (`.RowName` (break `DataTableRowHandle` _itemid)) (`self.PatronName`)) (> _quantity 0))
          (if (not (>= (`self.DispenserMagazine`) (`self.MaxDispenserMagazine`)))
            (`/Engine/EditorBlueprintResources/StandardMacros.IncrementInt` (`self.DispenserMagazine`)
              (:`  `
                (`/Engine/EditorBlueprintResources/StandardMacros.IncrementInt` (`self.Decrement Patrons Int`)
                  (:`  `
                    (`self.DecrementPatrons` (`.MainInventory` (break `AllItem` (`InventoryComponent.AllItems` (`self.GetComponentByClass` (`GameplayStatics.GetPlayerCharacter` 0) "/Script/ZombiSurvival.InventoryComponent")))) _array_index (`self.Decrement Patrons Int`))
                    (set `self.Decrement Patrons Int` 0)
                    (bind _aswbp_patron_bar (cast `/Game/UI/WidgetPlayer/PatronBar/WBP_PatronBar` (`PlayerInterface.PatronsBar` (`self.Player Interface`))))
                    (message `PatronsInterface.ReloadPatron` _aswbp_patron_bar (`self.DispenserMagazine`))
                    (break)))))))))))

(fn `UserConstructionScript`
  (`parent.UserConstructionScript`))