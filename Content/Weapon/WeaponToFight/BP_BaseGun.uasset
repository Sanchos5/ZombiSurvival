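; Base gun Blueprint handling firing effects, crosshair setup and magazine reloading from the player's inventory.
; BeginPlay caches the HUD crosshair, shaping it for shotgun or pistol via a class check on self.
; Shot adds muzzle flash, smoke and timeline-driven crosshair spread to the parent shot; ShotLineTrace is empty.
; Reload draws matching rounds from up to two inventory stack passes, then updates inventory UI and the ammo bar.
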(event `self.ReceiveBeginPlay`
  (bind _asbp_hud (cast `/Game/UI/BP_HUD` (`PlayerController.GetHUD` (`GameplayStatics.GetPlayerController` 0))))
  (bind _aswbp_interface_player (cast `/Game/UI/InterfaceGame/WBP_InterfacePlayer` (`/Game/UI/BP_HUD.PlayerInterface` _asbp_hud)))
  (bind _output_get (set `self.Player Interface` _aswbp_interface_player))
  (bind _output_get_2 (set `self.Crosshair` (`/Game/UI/InterfaceGame/WBP_InterfacePlayer.WBP_Crosshair` _output_get)))
  (if (== (`GameplayStatics.GetObjectClass` self) "/Game/Weapon/WeaponToFight/BP_shotgun.BP_Shotgun_C")
    ;[1 1 1] Crosshair for shotgun
    (set `/Game/UI/InterfaceGame/WBP_Crosshair.crosshair_spread` 40.0 _output_get_2)
    (set `/Game/UI/InterfaceGame/WBP_Crosshair.crosshair_thickness` 4.0 _output_get_2)
    (set `/Game/UI/InterfaceGame/WBP_Crosshair.crosshair_length` 30.0 _output_get_2)
    (else
      ;[1 1 1] Crosshair for pistol
      (set `/Game/UI/InterfaceGame/WBP_Crosshair.crosshair_spread` 10.0 _output_get_2)
      (set `/Game/UI/InterfaceGame/WBP_Crosshair.crosshair_thickness` 3.0 _output_get_2)
      (set `/Game/UI/InterfaceGame/WBP_Crosshair.crosshair_length` 15.0 _output_get_2)))
  (set `self.SpreadBeforeFire` (`/Game/UI/InterfaceGame/WBP_Crosshair.crosshair_spread` _output_get_2)))

(event `self.Shot`
  (bind _muzzleflash (`self.MuzzleFlash`))
  (bind _smokespawn (`self.SmokeSpawn`))
  (`parent.Shot`)
  (`NiagaraFunctionLibrary.SpawnSystemAtLocation` (`self.VFX MuzzleFlash`) (`SceneComponent.K2_GetComponentLocation` _muzzleflash) (`SceneComponent.K2_GetComponentRotation` _muzzleflash))
  (`NiagaraFunctionLibrary.SpawnSystemAtLocation` (`self.VFX Smoke`) (`SceneComponent.K2_GetComponentLocation` _smokespawn) (`SceneComponent.K2_GetComponentRotation` _smokespawn))
  (bind (_direction _crosshairspreadmultiplier) (`Timeline|CrosshairSpread` :!via `PlayFromStart`)
    (:`Update`
      (set `/Game/UI/InterfaceGame/WBP_Crosshair.crosshair_spread` (* _crosshairspreadmultiplier (`self.SpreadBeforeFire`)) (`self.Crosshair`)))))

(event `Reload`
  ;[1 1 1] Перезарядка
  (`self.ReloadDispenserMagazine`)
  (if (< (`self.DispenserMagazine`) (`self.MaxDispenserMagazine`))
    (`self.ReloadDispenserMagazine`))
  (bind _aswbp_patron_bar (cast `/Game/UI/WidgetPlayer/PatronBar/WBP_PatronBar` (`PlayerInterface.PatronsBar` (`self.Player Interface`))))
  (message `PatronsInterface.ReloadPatron` _aswbp_patron_bar (`self.DispenserMagazine`)))

(event `Play Reload Anim`
  (`SkeletalMeshComponent.PlayAnimation` (`self.WeaponMesh`) (`self.WeaponReloadAnim`) false))

(event `PlayFireAnim`
  (`SkeletalMeshComponent.PlayAnimation` (`self.WeaponMesh`) (`self.WeaponFireAnim`) false))

(fn `DecrementPatrons`
  (params (Array :type "Array of Slot Structure") (Index :type Integer) (IncrementInt :type Integer))
  (bind _index (`local.Index`))
  (bind (_itemid _quantity _itemtype) (break `Slot` (`|GetArrayItem` Array Index)))
  (bind _returnvalue (- _quantity IncrementInt))
  (if (> _returnvalue 0)
    (`KismetArrayLibrary.Array_Set` Array _index (make `Slot` _itemid _returnvalue _itemtype))
    (else
      (`KismetArrayLibrary.Array_Set` Array _index (make `Slot` (struct)))))
  (`InventoryComponent.UpdateAllInventoryUI` (`self.GetComponentByClass` (`GameplayStatics.GetPlayerCharacter` 0) "/Script/ZombiSurvival.InventoryComponent")))

(fn `ReloadDispenserMagazine`
  (for (_array_element _array_index) (`.MainInventory` (break `AllItem` (`InventoryComponent.AllItems` (`self.GetComponentByClass` (`GameplayStatics.GetPlayerCharacter` 0) "/Script/ZombiSurvival.InventoryComponent"))))
    (bind ((`ItemID` _itemid) (`Quantity` _quantity)) (break `Slot` _array_element))
    (if (and (== (`.RowName` (break `DataTableRowHandle` _itemid)) (`self.PatronName`)) (> _quantity 0))
      (for _ (range 1 (+ _quantity 1))
        (if (>= (`self.DispenserMagazine`) (`self.MaxDispenserMagazine`))
          (break)
          (else
            (`/Engine/EditorBlueprintResources/StandardMacros.IncrementInt` (`self.DispenserMagazine`)
              (:`  `
                (`/Engine/EditorBlueprintResources/StandardMacros.IncrementInt` (`self.Decrement Patrons Int`)))))))
      (`self.DecrementPatrons` (`.MainInventory` (break `AllItem` (`InventoryComponent.AllItems` (`self.GetComponentByClass` (`GameplayStatics.GetPlayerCharacter` 0) "/Script/ZombiSurvival.InventoryComponent")))) _array_index (`self.Decrement Patrons Int`))
      (set `self.Decrement Patrons Int` 0)
      (break))))

(fn `ShotLineTrace`
  (params (damage :type "Float (double-precision)")))

(fn `UserConstructionScript`)