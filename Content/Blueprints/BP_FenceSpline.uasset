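; Fence actor that lines a spline with instanced SM_Fence meshes, built in the construction script.
; It adds an instance at fixed distance steps along the spline and computes a look-at rotation from the previous piece to each new one.
; That look-at update leaves InstanceIndex unset, so it writes to the default instance rather than the previous one.
; The last instance takes its rotation from the closest spline point.
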(fn `UserConstructionScript`
  (bind _instancedstaticmesh (`self.InstancedStaticMesh`))
  (bind _returnvalue (- (`InstancedStaticMeshComponent.GetInstanceCount` (`self.InstancedStaticMesh`)) 1))
  (bind _outinstancetransform (`InstancedStaticMeshComponent.GetInstanceTransform` (`self.InstancedStaticMesh`) _returnvalue false))
  (`StaticMeshComponent.SetStaticMesh` (`self.InstancedStaticMesh`) "/Game/Environment/Meshes/SM_Fence.SM_Fence")
  (for _index (range (+ (`KismetMathLibrary.FFloor` (/ (`SplineComponent.GetSplineLength` (`self.Spline`)) 110.0)) 1))
    (bind _returnvalue_2 (`SplineComponent.GetLocationAtDistanceAlongSpline` (`self.Spline`) (* _index 110.0) "Local"))
    (`InstancedStaticMeshComponent.AddInstance` (`self.InstancedStaticMesh`) (`KismetMathLibrary.MakeTransform` _returnvalue_2) false)
    (if (> _index 0)
      (bind _outinstancetransform_2 (`InstancedStaticMeshComponent.GetInstanceTransform` _instancedstaticmesh (- _index 1) false))
      (`InstancedStaticMeshComponent.UpdateInstanceTransform` _instancedstaticmesh 0 (`KismetMathLibrary.MakeTransform` (.location _outinstancetransform_2) (`KismetMathLibrary.FindLookAtRotation` (.location _outinstancetransform_2) _returnvalue_2)) true false false)))
  (`InstancedStaticMeshComponent.UpdateInstanceTransform` (`self.InstancedStaticMesh`) _returnvalue (`KismetMathLibrary.MakeTransform` (.location _outinstancetransform) (`SplineComponent.FindRotationClosestToWorldLocation` (`self.Spline`) (.location _outinstancetransform) "Local")) false false false))