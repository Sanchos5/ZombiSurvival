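; BP_PlayStart is an actor that runs a media-based start screen before gameplay begins.
; On BeginPlay it disables player character input, shows WBP_Start with its MediaPlayer, and binds to that player's end-reached event.
; When the media ends, it removes the widget, reveals the BP_HUD player interface, restores input, calls AddSound on BP_BGSound, and destroys itself.
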(event `self.ReceiveBeginPlay`
  (bind _mediaplayer (`self.MediaPlayer`))
  (`self.DisableInput` (`GameplayStatics.GetPlayerCharacter` 0) (`GameplayStatics.GetPlayerController` 0))
  (bind _returnvalue (`|CreateWidget` "/Game/UI/WidgetPlayer/Start/WBP_Start.WBP_Start_C" null _mediaplayer))
  (`UserWidget.AddToViewport` _returnvalue 0)
  (add `MediaPlayer.OnEndReached` _mediaplayer (delegate `OnEndReached_Event`)))

(event `OnEndReached_Event`
  (`Widget.RemoveFromParent` (stale `self.ReceiveBeginPlay` _returnvalue))
  (bind _asbp_hud (cast `/Game/UI/BP_HUD` (`PlayerController.GetHUD` (`GameplayStatics.GetPlayerController` 0))))
  (`Widget.SetVisibility` (`HUDSurvival.PlayerInterface` _asbp_hud) "Visible")
  (`self.EnableInput` (`GameplayStatics.GetPlayerCharacter` 0) (`GameplayStatics.GetPlayerController` 0))
  (bind _returnvalue (`GameplayStatics.GetActorOfClass` "/Game/Blueprints/BP_BGSound.BP_BGSound_C"))
  (`/Game/Blueprints/BP_BGSound.AddSound` _returnvalue)
  (`self.K2_DestroyActor`))

(fn `UserConstructionScript`)