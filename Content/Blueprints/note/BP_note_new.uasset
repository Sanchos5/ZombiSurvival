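; Interactable note actor that opens a readable note on screen when the player interacts with it.
; Interact creates a WBP_note2 widget, adds it to the viewport, passes it the actor's ComicBook, Hat, Text and Ps content, then calls EStart on it.
; GetInteractText supplies the Russian "Read" prompt, and HideWidget always returns false.
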(event `InteractionInterface.Interact`
  (params (InstigatorPawn :type "Pawn Object Reference"))
  (bind _returnvalue (`|CreateWidget` "/Game/Blueprints/note/WBP_note2.WBP_note2_C"))
  (`UserWidget.AddToViewport` _returnvalue 0)
  (set `/Game/Blueprints/note/WBP_note2.wbp_comik_book` (`self.comic_book`) _returnvalue)
  (set `/Game/Blueprints/note/WBP_note2.hat_array` (`self.hat`) _returnvalue)
  (set `/Game/Blueprints/note/WBP_note2.Text_array` (`self.text`) _returnvalue)
  (set `/Game/Blueprints/note/WBP_note2.ps_array` (`self.ps`) _returnvalue)
  (`/Game/Blueprints/note/WBP_note2.E_start` _returnvalue))

(fn `GetInteractText`
  (returns (ReturnValue :type Text))
  (return "Прочитать"))

(fn `HideWidget`
  (returns (ReturnValue :type Boolean))
  (return false))

(fn `UserConstructionScript`)