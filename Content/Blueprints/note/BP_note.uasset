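; BP_note is an interactable note actor that the player reads, with the interaction prompt "Прочитать" (Read).
; On Interact it creates a WBP_note widget, fills it with the note's Hat, Text and Ps fields, and adds it to the viewport.
; It then passes its ComicBook reference to the widget.
; HideWidget always returns false, and the construction script is empty.
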(event `InteractionInterface.Interact`
  (params (InstigatorPawn :type "Pawn Object Reference"))
  (bind _returnvalue (`|CreateWidget` "/Game/Blueprints/note/WBP_note.WBP_note_C"))
  (`/Game/Blueprints/note/WBP_note.f_text` _returnvalue (`self.hat`) (`self.text`) (`self.ps`))
  (`UserWidget.AddToViewport` _returnvalue 0)
  (set `/Game/Blueprints/note/WBP_note.wbp_comik_book` (`self.comic_book`) _returnvalue))

(fn `GetInteractText`
  (returns (ReturnValue :type Text))
  (return "Прочитать"))

(fn `HideWidget`
  (returns (ReturnValue :type Boolean))
  (return false))

(fn `UserConstructionScript`)