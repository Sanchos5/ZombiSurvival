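; BP_key is an interactable key pickup that grants the player a door code.
; On interact it adds its Code to the player's CodeDoor collection, records its own name as a destroyed actor in the save system, then destroys itself.
; Highlight events toggle custom depth stencil on its cube mesh, and it supplies its own interaction prompt text.
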(event `InteractionInterface.Interact`
  (params (InstigatorPawn :type "Pawn Object Reference"))
  (bind _asbp_player (cast `/Game/Characters/Player/BP_Player` InstigatorPawn))
  (`KismetArrayLibrary.Array_Add` (`/Game/Characters/Player/BP_Player.code_door` _asbp_player) (`self.code`))
  (`SaveGameSystem.AddDestroyedActor` (subsystem `SaveGameSystem`) (`KismetSystemLibrary.GetObjectName` self))
  (`self.K2_DestroyActor`))

(event `InteractionInterface.HighlightActor`
  (bind _cube (`self.Cube`))
  (`PrimitiveComponent.SetRenderCustomDepth` _cube true)
  (`PrimitiveComponent.SetCustomDepthStencilValue` _cube 255))

(event `InteractionInterface.UnHighlightActor`
  (bind _cube (`self.Cube`))
  (`PrimitiveComponent.SetCustomDepthStencilValue` _cube 0)
  (`PrimitiveComponent.SetRenderCustomDepth` _cube false))

(fn `GetInteractText`
  (returns (ReturnValue :type Text))
  (return (`self.InteractionText`)))

(fn `HideWidget`
  (returns (ReturnValue :type Boolean))
  (return false))

(fn `UserConstructionScript`)