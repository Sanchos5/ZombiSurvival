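; BP_SurvivalGamemode is a game mode that triggers the start sequence when no save game is flagged.
; On BeginPlay, if the save game system's SaveGame value is false, it waits briefly, then hides the player interface through BP_HUD.
; It then spawns BP_PlayStart at the player character's transform.
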(event `self.ReceiveBeginPlay`
  (if (not (`SaveGameSystem.bSaveGame` (subsystem `SaveGameSystem`)))
    (`KismetSystemLibrary.Delay` 0.1)
    (bind _asbp_hud (cast `/Game/UI/BP_HUD` (`PlayerController.GetHUD` (`GameplayStatics.GetPlayerController` 0))))
    (`Widget.SetVisibility` (`HUDSurvival.PlayerInterface` _asbp_hud) "Hidden")
    (`|SpawnActorFromClass` "/Game/Blueprints/BP_PlayStart.BP_PlayStart_C" (`self.GetTransform` (`GameplayStatics.GetPlayerCharacter` 0)) "Undefined" "MultiplyWithRoot" null null)))

(fn `UserConstructionScript`)