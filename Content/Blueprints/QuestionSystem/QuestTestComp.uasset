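; Quest component (apparently a test version) that runs a sequential, DataTable-driven quest line and mirrors progress on the player HUD.
; On BeginPlay it loads quest rows, binds quest events and restores or starts quest data based on the save.
; UpdateQuest matches Reach, Iterate/Consume or Interact steps, then CompletedQuest advances the index or flags the next chapter.
; It also toggles subtitle hiding at specific quests and debug-prints saved indices on Tick.
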(event `self.ReceiveTick`
  (params (DeltaSeconds :type "Float (single-precision)"))
  (bind ((`CurrentQuestIndex` _currentquestindex) (`QuestData` _questdata) (`CurrentStepIndex` _currentstepindex)) (break `PlayerSaveData` (`BaseSaveGame.PlayerSaveData` (`SaveGameSystem.CurrentSaveGame` (subsystem `SaveGameSystem`)))))
  (`KismetSystemLibrary.Delay` 0.5)
  (`KismetSystemLibrary.PrintString` (`KismetStringLibrary.Conv_IntToString` _currentquestindex))
  (`KismetSystemLibrary.PrintString` (`KismetStringLibrary.Conv_IntToString` _currentstepindex)))

(event `QuestInterface.SetQuestDT`
  (params (Quest :type "DataTable Object Reference"))
  (bind _returnvalue (subsystem `SaveGameSystem`))
  (bind ((`Health` _health) (`CurrentQuestIndex` _currentquestindex) (`QuestData` _questdata) (`CurrentStepIndex` _currentstepindex)) (break `PlayerSaveData` (`BaseSaveGame.PlayerSaveData` (`SaveGameSystem.CurrentSaveGame` _returnvalue))))
  (bind _outrownames (`DataTableFunctionLibrary.GetDataTableRowNames` Quest))
  (bind _output_get (set `self.QuestNames` _outrownames))
  (for _array_element _output_get
    (bind _returnvalue_2 (`|GetDataTableRow` Quest _array_element)
      (:`then`
        (`KismetArrayLibrary.Array_AddUnique` (`self.QuestDataList`) _returnvalue_2)
        (add `self.OnQuestReached` (`|CreateDelegate` :!event `UpdateQuest`))
        (add `self.OnQuestItemIterated` (`|CreateDelegate` :!event `UpdateQuest`))
        (add `self.OnQuestItemInteract` (`|CreateDelegate` :!event `UpdateQuest`)))))
  (if (!= (`KismetTextLibrary.Conv_TextToString` (`.Description` (break `Quest` (`self.QuestData`)))) "")
    _
    (elif (== _health 0.0)
      (bind _output_get_2 (set `self.CurrentQuestIndex` 0))
      (set `self.QuestData` (`|GetArrayItem` (`self.QuestDataList`) _output_get_2))
      (elif (`SaveGameSystem.bSaveGame` _returnvalue)
        (set `self.CompletedStepsAmount` _currentstepindex)
        (bind _output_get_3 (set `self.QuestData` _questdata))
        (`self.OnUpdateWidget` _output_get_3)
        (else
          (bind _output_get_4 (set `self.CurrentQuestIndex` 0))
          (set `self.QuestData` (`|GetArrayItem` (`self.QuestDataList`) _output_get_4)))))))

(event `self.ReceiveBeginPlay`
  (`QuestInterface.SetQuestDT` (`self.QuestDataTable`))
  (bind _asbp_hud (cast `/Game/UI/BP_HUD` (`PlayerController.GetHUD` (`GameplayStatics.GetPlayerController` 0))))
  (bind _aswbp_interface_player (cast `/Game/UI/InterfaceGame/WBP_InterfacePlayer` (`/Game/UI/BP_HUD.PlayerInterface` _asbp_hud)))
  (set `self.Player Interface` _aswbp_interface_player))

(event `QuestInterface.UpdateQuest`
  (params (Type :type "EQuestType Enum (by ref)" :default "None") (Object :type "Actor Class Reference"))
  (bind _currentquestindex (`self.CurrentQuestIndex`))
  (`self.Compute Step Quest` Type Object)
  (if (>= (`self.CompletedStepsAmount`) (`self.InitialStepsAmount`))
    (`KismetSystemLibrary.Delay` 0.8)
    (`QuestInterface.CompletedQuest`)
    (if (or (== _currentquestindex 3) (== _currentquestindex 5) (== _currentquestindex 7))
      (set `/Game/Blueprints/QuestionSystem/Subtitles/SubtitlesComponent.bHideWidget` false (`/Game/Blueprints/QuestionSystem/Subtitles/BFL_Component.FindSubtitlesComp` (`GameplayStatics.GetPlayerCharacter` 0)))
      (else
        (set `/Game/Blueprints/QuestionSystem/Subtitles/SubtitlesComponent.bHideWidget` true (`/Game/Blueprints/QuestionSystem/Subtitles/BFL_Component.FindSubtitlesComp` (`GameplayStatics.GetPlayerCharacter` 0)))))))

(event `self.StartQuest`
  (bind _wbp_quest (`/Game/UI/InterfaceGame/WBP_InterfacePlayer.WBP_Quest` (`self.Player Interface`)))
  (bind (_reach _iterate _interact) (break `QuestSteps` (`.Steps` (break `Quest` (`self.QuestData`)))))
  (set `self.InitialStepsAmount` (+ (`KismetArrayLibrary.Array_Length` _reach) (`KismetArrayLibrary.Array_Length` _iterate) (`KismetArrayLibrary.Array_Length` _interact)) :!label _label)
  (`/Engine/EditorBlueprintResources/StandardMacros.IsValid` _wbp_quest
    (:`Is Valid`
      (`/Game/UI/Quest/WBP_Quest.OnUpdateWidget_Event` _wbp_quest (`self.QuestData`)))))

(event `NextQuest`
  (set `self.QuestData` (`|GetArrayItem` (`self.QuestDataList`) (`self.CurrentQuestIndex`)))
  (goto _label))

(event `QuestInterface.CompletedQuest`
  (if (`self.Completed`)
    (`/Game/UI/Quest/WBP_Quest.CompleteQuest` (`/Game/UI/InterfaceGame/WBP_InterfacePlayer.WBP_Quest` (`self.Player Interface`)))
    (set `self.CompletedStepsAmount` 0)
    (`/Engine/EditorBlueprintResources/StandardMacros.IncrementInt` (`self.CurrentQuestIndex`)
      (:`  `
        (if (not (> (`self.CurrentQuestIndex`) (`KismetArrayLibrary.Array_LastIndex` (`self.QuestDataList`))))
          (`KismetSystemLibrary.K2_SetTimerDelegate` (`|CreateDelegate` :!event `NextQuest`) 0.02)
          (else
            (set `self.Go Next Chapter` true)))))))

(fn `Compute Step Quest`
  (params (Type :type "EQuestType Enum" :default "None") (Object :type "Actor Class Reference") (`Quest ID` :type String))
  (locals (IterationIndex :type Integer) (ReachIndex :type Integer) (InteractIndex :type Integer) (IterationAmount :type Integer))
  (bind (_reach _iterate _interact) (break `QuestSteps` (`.Steps` (break `Quest` (`self.QuestData`)))))
  (switch `EQuestType` Type
    (:`Iterate`
      (if (> (`KismetArrayLibrary.Array_Length` _iterate) 0) :!label _label
        (switch `EQuestType` (`local.Type`) :!label _label_2
          (:`Iterate`
            (for (_array_element _array_index) (`.Iterate` (break `QuestSteps` (`.Steps` (break `Quest` (`self.QuestData`))))) :!label _label_3
              (set `local.IterationIndex` _array_index)
              (bind (_description _objects _itemtype _bcompleted _currentamount _maxamount _type) (break `QuestIterate` _array_element))
              (if (and (== _objects "/Game/Blueprints/Inventory/Blueprints/BP_InventoryItem.BP_InventoryItem_C") (not _bcompleted) (`|EnumEquality` _type (`local.Type`)) (`|EnumEquality` _itemtype (`self.ItemType`)))
                (bind _output_get (set `local.IterationAmount` (+ _currentamount 1)))
                (setmembers `QuestIterate` :`StructRef` (`|GetArrayItem` (`.Iterate` (break `QuestSteps` (`.Steps` (break `Quest` (`self.QuestData`))))) (`local.IterationIndex`)) :`CurrentAmount` _output_get)
                (if (>= (`local.IterationAmount`) _maxamount)
                  (bind _output_get_2 (set `self.Completed` true))
                  (bind _structout (setmembers `QuestIterate` :`StructRef` (`|GetArrayItem` (`.Iterate` (break `QuestSteps` (`.Steps` (break `Quest` (`self.QuestData`))))) (`local.IterationIndex`)) :`bCompleted` _output_get_2))
                  (`/Engine/EditorBlueprintResources/StandardMacros.IncrementInt` (`self.CompletedStepsAmount`)
                    (:`  `
                      _)))
                (`/Game/UI/Quest/WBP_Quest.UpdateStep` (`/Game/UI/InterfaceGame/WBP_InterfacePlayer.WBP_Quest` (`self.Player Interface`)) (`KismetTextLibrary.Conv_TextToString` (`.Description` (break `QuestIterate` _structout)))))))
          (:`Interact`
            (for (_array_element_2 _array_index_2) (`.Interact` (break `QuestSteps` (`.Steps` (break `Quest` (`self.QuestData`)))))
              (set `local.InteractIndex` _array_index_2)
              (bind (_description_2 _objects_2 _bcompleted_2 _type_2) (break `QuestInteract` _array_element_2))
              (if (and (== _objects_2 (`local.Object`)) (not _bcompleted_2) (`|EnumEquality` _type_2 (`local.Type`)))
                (bind _output_get_3 (set `self.Completed` true))
                (bind _structout_2 (setmembers `QuestInteract` :`StructRef` (`|GetArrayItem` (`.Interact` (break `QuestSteps` (`.Steps` (break `Quest` (`self.QuestData`))))) (`local.InteractIndex`)) :`bCompleted` _output_get_3))
                (`/Game/UI/Quest/WBP_Quest.UpdateStep` (`/Game/UI/InterfaceGame/WBP_InterfacePlayer.WBP_Quest` (`self.Player Interface`)) (`KismetTextLibrary.Conv_TextToString` (`.Description` (break `QuestInteract` _structout_2))))
                (`/Engine/EditorBlueprintResources/StandardMacros.IncrementInt` (`self.CompletedStepsAmount`)))))
          (:`Reach`
            (for (_array_element_3 _array_index_3) (`.Reach` (break `QuestSteps` (`.Steps` (break `Quest` (`self.QuestData`)))))
              (set `local.ReachIndex` _array_index_3)
              (bind (_description_3 _reached _reachid _bcompleted_3 _type_3) (break `QuestReach` _array_element_3))
              (if (and (== _reached (`self.Reach`)) (not _bcompleted_3) (`|EnumEquality` _type_3 (`local.Type`)) (`KismetStringLibrary.EqualEqual_StrStr` _reachid (`self.QuestID`)))
                (bind _output_get_4 (set `self.Completed` true))
                (bind _structout_3 (setmembers `QuestReach` :`StructRef` (`|GetArrayItem` (`.Reach` (break `QuestSteps` (`.Steps` (break `Quest` (`self.QuestData`))))) (`local.ReachIndex`)) :`bCompleted` _output_get_4))
                (`/Game/UI/Quest/WBP_Quest.UpdateStep` (`/Game/UI/InterfaceGame/WBP_InterfacePlayer.WBP_Quest` (`self.Player Interface`)) (`KismetTextLibrary.Conv_TextToString` (`.Description` (break `QuestReach` _structout_3))))
                (`/Engine/EditorBlueprintResources/StandardMacros.IncrementInt` (`self.CompletedStepsAmount`)))))
          (:`Consume`
            (goto _label_3)))))
    (:`Interact`
      (if (> (`KismetArrayLibrary.Array_Length` _interact) 0)
        (goto _label_2)))
    (:`Reach`
      (if (> (`KismetArrayLibrary.Array_Length` _reach) 0)
        (goto _label_2)))
    (:`Consume`
      (goto _label))))