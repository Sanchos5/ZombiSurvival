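; Trigger actor that reports a Reach quest objective when the player enters its box.
; On a BP_Player overlap it writes its ReachID to the player's quest component, then calls the quest-reached notification with the Reach type and its own class.
; If the current quest index then matches TestIndex, a DoOnce changes the player's subtitles to IndexSub a single time.
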(event `self.Box.OnComponentBeginOverlap`
  (params (OverlappedComponent :type "PrimitiveComponent Object Reference") (OtherActor :type "Actor Object Reference") (OtherComp :type "PrimitiveComponent Object Reference") (OtherBodyIndex :type Integer) (bFromSweep :type Boolean) (SweepResult :type "HitResult Structure (by ref)"))
  (bind _returnvalue (`QuestComponent.FindQuestComponent` (`GameplayStatics.GetPlayerCharacter` 0)))
  (cast `/Game/Characters/Player/BP_Player` OtherActor)
  (set `QuestComponent.QuestID` (`self.ReachID`) _returnvalue)
  (`QuestComponent.OnQuestReached` _returnvalue "Reach" (`GameplayStatics.GetObjectClass` self))
  (if (== (`QuestComponent.CurrentQuestIndex` (`QuestComponent.FindQuestComponent` (`GameplayStatics.GetPlayerCharacter` 0))) (`self.TestIndex`))
    (`/Engine/EditorBlueprintResources/StandardMacros.DoOnce` false
      (:`Completed`
        (`/Game/Blueprints/QuestionSystem/Subtitles/SubtitlesComponent.ChangeSubtitles` (`/Game/Blueprints/QuestionSystem/Subtitles/BFL_Component.FindSubtitlesComp` (`GameplayStatics.GetPlayerCharacter` 0)) (`self.Index Sub`))))))

(fn `UserConstructionScript`)