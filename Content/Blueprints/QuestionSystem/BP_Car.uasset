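; Interactable car for the quest system that reports player interaction to the quest component as an Interact event with its own class.
; When the quest index then matches the subtitle index, it triggers a subtitle change and plays a failed engine start sound, or a successful one at a single hardcoded quest step.
; It supplies a Russian interaction prompt and hides its widget outside a few hardcoded quest steps.
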(event `InteractionInterface.Interact`
  (params (InstigatorPawn :type "Pawn Object Reference"))
  (bind _returnvalue (`self.K2_GetActorLocation`))
  (bind _returnvalue_2 (`/Game/Blueprints/QuestionSystem/Subtitles/BFL_Component.FindSubtitlesComp` (`GameplayStatics.GetPlayerCharacter` 0)))
  (bind _currentquestindex (`QuestComponent.CurrentQuestIndex` (`QuestComponent.FindQuestComponent` (`GameplayStatics.GetPlayerCharacter` 0))))
  (bind _currentindex (`/Game/Blueprints/QuestionSystem/Subtitles/SubtitlesComponent.CurrentIndex` _returnvalue_2))
  (bind _asbp_player (cast `/Game/Characters/Player/BP_Player` InstigatorPawn))
  (`QuestComponent.OnQuestItemInteract` (`QuestComponent.FindQuestComponent` _asbp_player) "Interact" (`GameplayStatics.GetObjectClass` self))
  (if (== _currentquestindex _currentindex)
    (`/Game/Blueprints/QuestionSystem/Subtitles/SubtitlesComponent.ChangeSubtitles` _returnvalue_2 _currentindex)
    (if (!= _currentquestindex 7)
      (`GameplayStatics.PlaySoundAtLocation` "/Game/Sounds/Car/WAV_Engine_Start_Failed.WAV_Engine_Start_Failed" _returnvalue (struct) 1.0 1.0 0.0 null null null null)
      (else
        (`GameplayStatics.PlaySoundAtLocation` "/Game/Sounds/Car/WAV_Engine_Start.WAV_Engine_Start" _returnvalue (struct) 1.0 1.0 0.0 null null null null)))))

(fn `GetInteractText`
  (returns (ReturnValue :type Text))
  (return "Взаимодействовать"))

(fn `HideWidget`
  (returns (ReturnValue :type Boolean))
  (bind _currentquestindex (`QuestComponent.CurrentQuestIndex` (`QuestComponent.FindQuestComponent` (`GameplayStatics.GetPlayerCharacter` 0))))
  (if (or (== _currentquestindex 4) (== _currentquestindex 6) (== _currentquestindex 8))
    (return false)
    (else
      (return true))))

(fn `UserConstructionScript`)