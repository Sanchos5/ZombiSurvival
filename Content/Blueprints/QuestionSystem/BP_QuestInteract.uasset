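; BP_QuestInteract is an interactable quest item that the player picks up when its class matches an Interact step in their quest data.
; Pickup destroys the actor, plays a sound and reports the interaction to the player's quest component.
; If only one of Quest1 or Quest2 is valid, that one teleports its Key and Contejner to offsets from itself.
; Completed-step counts and the canister class trigger subtitle changes.
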(event `InteractionInterface.Interact`
  (params (InstigatorPawn :type "Pawn Object Reference"))
  (bind _returnvalue (`GameplayStatics.GetObjectClass` self))
  (bind _asbp_player (cast `/Game/Characters/Player/BP_Player` InstigatorPawn))
  (bind _returnvalue_2 (`QuestComponent.FindQuestComponent` _asbp_player))
  (for _array_element (`.Interact` (break `QuestSteps` (`.Steps` (break `Quest` (`QuestComponent.QuestData` _returnvalue_2)))))
    (bind (_description _objects) (break `QuestInteract` _array_element))
    (if (== _objects _returnvalue)
      (`self.f_valid`)
      (`self.K2_DestroyActor`)
      (`GameplayStatics.PlaySound2D` "/Game/Sounds/Consumables/WAV_Item_Pickup.WAV_Item_Pickup" 1.0 1.0 0.0 null null)
      (`QuestComponent.OnQuestItemInteract` _returnvalue_2 "Interact" _returnvalue)
      (if (== (`QuestComponent.CompletedStepsAmount` _returnvalue_2) 3)
        (`/Engine/EditorBlueprintResources/StandardMacros.DoOnce` false
          (:`Completed`
            (`/Game/Blueprints/QuestionSystem/Subtitles/SubtitlesComponent.ChangeSubtitles` (`/Game/Blueprints/QuestionSystem/Subtitles/BFL_Component.FindSubtitlesComp` (`GameplayStatics.GetPlayerCharacter` 0)) 4)))
        (elif (and (== _objects "/Game/Blueprints/QuestionSystem/BP_QuestCanister.BP_QuestCanister_C") (== (`QuestComponent.CompletedStepsAmount` (`QuestComponent.FindQuestComponent` (`GameplayStatics.GetPlayerCharacter` 0))) 1))
          (`/Game/Blueprints/QuestionSystem/Subtitles/SubtitlesComponent.ChangeSubtitles` (`/Game/Blueprints/QuestionSystem/Subtitles/BFL_Component.FindSubtitlesComp` (`GameplayStatics.GetPlayerCharacter` 0)) 6))))))

(fn `f_spawn`
  (`self.K2_SetActorLocation` (`self.key`) (+ (`self.K2_GetActorLocation`) (`self.local_spawn_key`)) false true)
  (`self.K2_SetActorLocation` (`self.contejner`) (+ (`self.K2_GetActorLocation`) (`self.local_spawn_contejner`)) false true))

(fn `f_valid`
  (bind _quest1 (`self.quest1`))
  (bind _quest2 (`self.quest2`))
  (`/Engine/EditorBlueprintResources/StandardMacros.IsValid` _quest1
    (:`Is Valid`
      (`/Engine/EditorBlueprintResources/StandardMacros.IsValid` _quest2
        (:`Is Not Valid`
          (`self.f_spawn` _quest1))))
    (:`Is Not Valid`
      (`/Engine/EditorBlueprintResources/StandardMacros.IsValid` _quest2
        (:`Is Valid`
          (`self.f_spawn` _quest2))))))

(fn `GetInteractText`
  (returns (ReturnValue :type Text))
  (return ""))

(fn `HideWidget`
  (returns (ReturnValue :type Boolean))
  (return false))

(fn `UserConstructionScript`)