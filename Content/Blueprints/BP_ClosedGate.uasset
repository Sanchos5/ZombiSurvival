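; BP_ClosedGate is an interactable gate that can be locked and requires the player to hold a matching code.
; On Interact, CheckPlayerKey looks for the gate's Code in BP_Player's CodeDoor and clears Closed if found.
; Without the code, it plays a locked-door sound and shows a WBP_door widget.
; An unlocked gate passes the interaction to the parent class's Interact logic.
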(event `InteractionInterface.Interact`
  (params (InstigatorPawn :type "Pawn Object Reference"))
  (bind _output_get (`self.CheckPlayerKey` InstigatorPawn "/Game/UI/InterfaceGame/WBP_door.WBP_door_C"))
  (if (not _output_get)
    (`parent.Interact` InstigatorPawn)))

(fn `CheckPlayerKey`
  (params (Object :type "Object Object Reference") (Class :type "UserWidget Class Reference"))
  (returns (Output_Get :type Boolean))
  (if (`self.Closed?`)
    (bind _asbp_player (cast `/Game/Characters/Player/BP_Player` Object))
    (if (`KismetArrayLibrary.Array_Contains` (`/Game/Characters/Player/BP_Player.code_door` _asbp_player) (`self.code`))
      (bind _output_get (set `self.Closed?` false))
      (return _output_get)
      (else
        (`GameplayStatics.PlaySound2D` "/Game/Sounds/WAV_Door_Closed.WAV_Door_Closed" 1.0 1.0 0.0 null null)
        (bind _returnvalue (`|CreateWidget` Class))
        (`UserWidget.AddToViewport` _returnvalue 0)
        (return true)))))

(fn `UserConstructionScript`
  (`parent.UserConstructionScript`))