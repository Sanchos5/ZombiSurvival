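; BP_SpawnZombie is a placeable spawner that creates one batch of MaxCurrentZombie zombies, either at BeginPlay or when triggered.
; With IsTrigger off it spawns immediately; otherwise a BP_Player entering the Box triggers it, with a shared DoOnce preventing repeats.
; Each zombie gets a random yaw and a random reachable point within SphereRadius of the actor's origin, not the offset Sphere.
; The construction script positions and sizes Sphere and Box from variables.
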(event `self.ReceiveBeginPlay`
  (if (not (`self.IsTrigger`))
    (`/Engine/EditorBlueprintResources/StandardMacros.DoOnce` false :!label _label
      (:`Completed`
        (for _ (range (`self.Max Current Zombie`))
          (`self.Spawner`))))))

(event `SpawnZombieBeginOverlap`
  (if (`self.IsTrigger`)
    (goto _label)))

(event `self.Box.OnComponentBeginOverlap`
  (params (OverlappedComponent :type "PrimitiveComponent Object Reference") (OtherActor :type "Actor Object Reference") (OtherComp :type "PrimitiveComponent Object Reference") (OtherBodyIndex :type Integer) (bFromSweep :type Boolean) (SweepResult :type "HitResult Structure (by ref)"))
  (cast `/Game/Characters/Player/BP_Player` OtherActor)
  (set `self.IsTrigger` true)
  (`self.SpawnZombieBeginOverlap`))

(fn `Spawner`
  (`|SpawnActorFromClass` "/Game/Characters/Enemy/BP_Zombie_NewAnimation.BP_Zombie_NewAnimation_C" (`KismetMathLibrary.MakeTransform` (`NavigationSystemV1.K2_GetRandomReachablePointInRadius` (`self.K2_GetActorLocation`) (`self.Sphere Radius`) null null) (`KismetMathLibrary.MakeRotator` 0.0 0.0 (`KismetMathLibrary.RandomFloatInRange` 0.0 360.0))) "AdjustIfPossibleButAlwaysSpawn" "MultiplyWithRoot" null null))

(fn `UserConstructionScript`
  (bind _sphere (`self.Sphere`))
  (`SphereComponent.SetSphereRadius` _sphere (`self.Sphere Radius`) true)
  (`SceneComponent.K2_SetRelativeLocation` _sphere (`self.LocationSpawnZombie`) false false)
  (`SceneComponent.K2_SetRelativeLocation` (`self.Box`) (`self.LocationTrigger`) false false)
  (`SceneComponent.SetRelativeScale3D` (`self.Box`) (`self.TriggerTransform`)))