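; Interactable world pickup for an inventory item, with mesh and item type filled from a data table on construction and on load.
; A secondary mesh shows only when the item matches the vodka row.
; Interact adds the item to the instigator's inventory, refreshing the HUD ammo bar for Patrons items.
; On success it destroys itself, updates inventory UI, registers as destroyed with the game instance and notifies the player's quest component.
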(event `self.ReceiveBeginPlay`
  (bind _secondsm (`self.SecondSM`))
  (bind _item_itemid (break `Slot` (`self.Item`)))
  (bind _vodka_item_itemid (break `Slot` (`self.Vodka_Item`)))
  (if (== (`.RowName` (break `DataTableRowHandle` _item_itemid)) (`.RowName` (break `DataTableRowHandle` _vodka_item_itemid)))
    (`SceneComponent.SetVisibility` _secondsm true false)
    (else
      (`SceneComponent.SetVisibility` _secondsm false false))))

(event `InteractionInterface.Interact`
  (params (InstigatorPawn :type "Pawn Object Reference"))
  (bind _item (`self.Item`))
  (bind _returnvalue (`QuestComponent.FindQuestComponent` (`GameplayStatics.GetPlayerCharacter` 0)))
  (bind _output_get (set `self.PlayerInventory` (`self.GetComponentByClass` InstigatorPawn "/Script/ZombiSurvival.InventoryComponent")))
  (`/Engine/EditorBlueprintResources/StandardMacros.IsValid` _output_get
    (:`Is Valid`
      (bind _returnvalue_2 (`InventoryComponent.AddToInventory` (`self.PlayerInventory`) _item))
      (if _returnvalue_2
        (if (`|EnumEquality` (`.ItemType` (break `Slot` _item)) "EI_Patrons")
          (bind _asbp_hud (cast `/Game/UI/BP_HUD` (`PlayerController.GetHUD` (`GameplayStatics.GetPlayerController` 0))))
          (bind _aswbp_patron_bar (cast `/Game/UI/WidgetPlayer/PatronBar/WBP_PatronBar` (`/Game/UI/InterfaceGame/WBP_InterfacePlayer.PatronsBar` (`/Game/UI/BP_HUD.PlayerInterface` _asbp_hud))))
          (`/Game/UI/WidgetPlayer/PatronBar/WBP_PatronBar.PatronsInInventory` _aswbp_patron_bar))
        (`self.K2_DestroyActor`)
        (`InventoryComponent.UpdateAllInventoryUI` (`self.PlayerInventory`))
        (`BaseGameInstance.AddDestroyedActor` (subsystem `BaseGameInstance`) self)
        (set `QuestComponent.ItemType` (`.ItemType` (break `Slot` (`self.Item`))) _returnvalue)
        (`QuestComponent.OnQuestItemIterated` _returnvalue "Iterate" (`GameplayStatics.GetObjectClass` self))))))

(event `SavalableObjectInterface.OnActorLoaded`
  (`self.Initialize Item`))

(fn `GetInteractText`
  (returns (ReturnValue :type Text))
  (return (`self.InteractionText`)))

(fn `HideWidget`
  (returns (ReturnValue :type Boolean))
  (return false))

(fn `Initialize Item`
  (bind (_item_itemid _item_quantity) (break `Slot` (`self.Item`)))
  (bind _item_itemid_2 (break `Slot` (`self.Item`)))
  (bind _returnvalue (`|GetDataTableRow` (`self.Item Data Table`) (`.RowName` (break `DataTableRowHandle` _item_itemid_2)))
    (:`then`
      (bind ((`ItemType` _itemtype) (`Mesh` _mesh)) (break `ItemInfo` _returnvalue))
      (`StaticMeshComponent.SetStaticMesh` (`self.StaticMesh`) _mesh)
      (set `self.Item` (make `Slot` _item_itemid _item_quantity _itemtype)))))

(fn `UserConstructionScript`
  (`self.Initialize Item`))