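; BP_InventoryItem is a world pickup actor that adds its item to the player's inventory when interacted with.
; The construction script looks up the item's ID in ItemDataTable and sets the static mesh from that row.
; On Interact, it calls AddToInventory on the player character's InventoryComponent; on success it destroys itself and refreshes the melee, ranged or eatables UI by item type, plus the main inventory UI.
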(event `InteractionInterface.Interact`
  (params (InstigatorPawn :type "Pawn Object Reference"))
  (bind _item (`self.Item`))
  (bind _playerinventory (`self.PlayerInventory`))
  (bind _output_get (set `self.PlayerInventory` (`self.GetComponentByClass` (`GameplayStatics.GetPlayerCharacter` 0) "/Script/ZombiSurvival.InventoryComponent")))
  (`/Engine/EditorBlueprintResources/StandardMacros.IsValid` _output_get
    (:`Is Valid`
      (bind _returnvalue (`InventoryComponent.AddToInventory` (`self.PlayerInventory`) _item))
      (if _returnvalue
        (`self.K2_DestroyActor`)
        (switch `EItemType` (`.ItemType` (break `Slot` _item))
          (:`EI_MeleeWeapon`
            (`InventoryComponent.UpdateMeleeWeaponUI` _playerinventory))
          (:`EI_RangeWeapon`
            (`InventoryComponent.UpdateRangeWeaponUI` _playerinventory))
          (:`EI_Eatables`
            (`InventoryComponent.UpdateEatablesUI` _playerinventory)))
        (`InventoryComponent.UpdateMainInventoryUI` _playerinventory)))))

(fn `UserConstructionScript`
  (bind _returnvalue (`|GetDataTableRow` (`self.Item Data Table`) (`.RowName` (break `DataTableRowHandle` (break `Slot` (`self.Item`)))))
    (:`then`
      (`StaticMeshComponent.SetStaticMesh` (`self.StaticMesh`) (`.Mesh` (break `ItemInfo` _returnvalue))))))