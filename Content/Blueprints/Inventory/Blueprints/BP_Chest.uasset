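; BP_Chest is an interactable chest that opens an inventory screen when the player interacts with it.
; Interact refreshes the player and chest panels through its ChestInventory component, shows that component's widget, and switches to UI-only input with a visible cursor.
; It also hides the player's InteractionComponent prompt, printing a message if that widget is invalid.
; GetInteractText returns empty text and HideWidget returns false.
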(event `InteractionInterface.Interact`
  (params (InstigatorPawn :type "Pawn Object Reference"))
  (bind _returnvalue (`GameplayStatics.GetPlayerController` 0))
  (bind _chestinventory (`self.ChestInventory`))
  (bind _chestinventorywidget (`ChestInventoryComponent.ChestInventoryWidget` _chestinventory))
  (`ChestInventoryComponent.UpdatePlayerInventoryUI` _chestinventory)
  (`ChestInventoryComponent.UpdateChestInventoryUI` _chestinventory)
  (`Widget.SetVisibility` _chestinventorywidget "Visible")
  (`WidgetBlueprintLibrary.SetInputMode_UIOnlyEx` _returnvalue _chestinventorywidget)
  (set `PlayerController.bShowMouseCursor` true _returnvalue)
  (bind _interactionwidget (`InteractionComponent.InteractionWidget` (`self.GetComponentByClass` (`GameplayStatics.GetPlayerCharacter` 0) "/Script/ZombiSurvival.InteractionComponent"))
    (:`then`
      (`Widget.SetVisibility` _interactionwidget "Hidden"))
    (:`else`
      (`KismetSystemLibrary.PrintString` "Interaction Widget is not vailable"))))

(fn `GetInteractText`
  (returns (ReturnValue :type Text))
  (return ""))

(fn `HideWidget`
  (returns (ReturnValue :type Boolean))
  (return false))

(fn `UserConstructionScript`)