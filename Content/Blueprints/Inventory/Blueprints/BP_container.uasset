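; BP_container is an interactable chest that opens an inventory screen for the player.
; On Interact it creates a chest inventory widget with itself as owner, has its ChestInventory refresh player and chest views, and plays an open sound.
; Input switches to UI-only with a visible cursor.
; It supplies the Russian "Open" prompt and a Hide flag, set on opening and returned by HideWidget.
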(event `InteractionInterface.Interact`
  (params (InstigatorPawn :type "Pawn Object Reference"))
  (bind _returnvalue (`GameplayStatics.GetPlayerController` 0))
  (bind _chestinventory (`self.ChestInventory`))
  (bind _returnvalue_2 (`|CreateWidget` "/Game/Blueprints/Inventory/Widgets/ChestWidget/WBP_ChestInventory.WBP_ChestInventory_C"))
  (bind _output_get (set `ChestInventoryComponent.ChestInventoryWidget` _returnvalue_2 (`self.ChestInventory`)))
  (set `ChestInventoryWidget.ChestOwner` self _output_get)
  (`UserWidget.AddToViewport` _output_get 0)
  (`ChestInventoryComponent.UpdatePlayerInventoryUI` _chestinventory)
  (`ChestInventoryComponent.UpdateChestInventoryUI` _chestinventory)
  (`WidgetBlueprintLibrary.SetInputMode_UIOnlyEx` _returnvalue (`ChestInventoryComponent.ChestInventoryWidget` _chestinventory))
  (set `PlayerController.bShowMouseCursor` true _returnvalue)
  (set `self.Hide` true)
  (`GameplayStatics.PlaySound2D` "/Game/Sounds/WAV_Chest_Open.WAV_Chest_Open" 1.0 1.0 0.0 null null))

(fn `GetInteractText`
  (returns (ReturnValue :type Text))
  (return "Открыть"))

(fn `HideWidget`
  (returns (ReturnValue :type Boolean))
  (return (`self.Hide`)))

(fn `UserConstructionScript`)