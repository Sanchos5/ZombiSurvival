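; BPC_WorldMap is a component that converts world locations into positions on the player HUD's map widget.
; On BeginPlay it caches the map from WBP_InterfacePlayer along with the player marker's size.
; Two corner actors define the world bounds, used to normalize locations, scale them to map size and center the marker.
; A function moves and yaw-rotates the player marker, but its call in the event graph is disconnected.
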(event `self.ReceiveBeginPlay`
  (bind _asbp_hud (cast `/Game/UI/BP_HUD` (`PlayerController.GetHUD` (`GameplayStatics.GetPlayerController` 0))))
  (bind _aswbp_interface_player (cast `/Game/UI/InterfaceGame/WBP_InterfacePlayer` (`/Game/UI/BP_HUD.PlayerInterface` _asbp_hud)))
  (bind _output_get (set `self.Interface Player` _aswbp_interface_player))
  (set `self.Map` (`/Game/UI/InterfaceGame/WBP_InterfacePlayer.WBP_Map` _output_get))
  (bind _map (`self.Map`)
    (:`then`
      (set `self.OriginalPlayerSize` (`KismetMathLibrary.MakeVector2D` (`KismetMathLibrary.Conv_IntToDouble` (`/Game/UI/Map/WBP_Map.PlayerSizeX` _map)) (`KismetMathLibrary.Conv_IntToDouble` (`/Game/UI/Map/WBP_Map.PlayerSizeY` _map)))))
    (:`else`)))

(event `InitializeMap`
  (params (Player :type "Character Object Reference"))
  (`/Engine/EditorBlueprintResources/StandardMacros.IsValid` Player
    (:`Is Valid`
      (set `self.Player` Player))))

(fn `ConvertLocationToMapLocation`
  (params (Location :type "Vector Structure"))
  (returns (Out :type "Vector2D Structure"))
  (bind (_returnvalue_x _returnvalue_y) (`KismetMathLibrary.BreakVector` (`Actor.K2_GetActorLocation` (`self.UpperLeftCorner`))))
  (return (`KismetMathLibrary.MakeVector2D` (`KismetMathLibrary.Abs` (- (.x Location) _returnvalue_x)) (`KismetMathLibrary.Abs` (- (.y Location) _returnvalue_y)))))

(fn `GetMapHeigh`
  (returns (Out :type "Float (double-precision)"))
  (return (`KismetMathLibrary.Abs` (- (.y (`Actor.K2_GetActorLocation` (`self.LowerRightCorner`))) (.y (`Actor.K2_GetActorLocation` (`self.UpperLeftCorner`)))))))

(fn `GetMapWidth`
  (returns (Out :type "Float (double-precision)"))
  (return (`KismetMathLibrary.Abs` (- (.x (`Actor.K2_GetActorLocation` (`self.LowerRightCorner`))) (.x (`Actor.K2_GetActorLocation` (`self.UpperLeftCorner`)))))))

(fn `LocationToMapPosition`
  (params (Location :type "Vector Structure") (WidgetSize :type "Vector2D Structure"))
  (returns (Out :type "Vector2D Structure"))
  (bind (_x _y) (`KismetMathLibrary.BreakVector2D` WidgetSize))
  (bind _map (`self.Map`))
  (bind (_x_2 _y_2) (`KismetMathLibrary.BreakVector2D` (`self.ConvertLocationToMapLocation` Location)))
  (return (`KismetMathLibrary.MakeVector2D` (- (* (/ _x_2 (`self.GetMapWidth`)) (`/Game/UI/Map/WBP_Map.MapSizeX` _map)) (/ _x 2.0)) (- (* (/ _y_2 (`self.GetMapHeigh`)) (`/Game/UI/Map/WBP_Map.MapSizeY` _map)) (/ _y 2.0)))))

(fn `UpdatePlayerPositionOnMap`
  (bind (_returnvalue_roll _returnvalue_pitch _returnvalue_yaw) (`KismetMathLibrary.BreakRotator` (`Actor.K2_GetActorRotation` (`GameplayStatics.GetPlayerCharacter` 0))))
  (bind _sizebox_player (`/Game/UI/Map/WBP_Map.SizeBox_Player` (`self.Map`)))
  (`Widget.SetRenderTranslation` _sizebox_player (`self.LocationToMapPosition` (`Actor.K2_GetActorLocation` (`self.Player`)) (`self.OriginalPlayerSize`)))
  (`Widget.SetRenderTransformAngle` _sizebox_player (- _returnvalue_yaw 90.0))
  (return))