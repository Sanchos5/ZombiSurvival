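; BP_PlayEnd runs the game's ending screen and returns to the menu level when its media finishes.
; On BeginPlay it removes the BP_BGSound background audio, stops stat handling on the player's PlayerStatsComponent, and shows a WBP_End widget fed with the MediaPlayer.
; The MediaPlayer's OnEndReached event removes that widget and opens LVL_menu.
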(event `self.ReceiveBeginPlay`
  (bind _mediaplayer (`self.MediaPlayer`))
  (bind _returnvalue (`GameplayStatics.GetActorOfClass` "/Game/Blueprints/BP_BGSound.BP_BGSound_C"))
  (`/Game/Blueprints/BP_BGSound.DestroyComponent` _returnvalue)
  (`PlayerStatsComponent.StopHandleStats` (`self.GetComponentByClass` (`GameplayStatics.GetPlayerCharacter` 0) "/Script/ZombiSurvival.PlayerStatsComponent"))
  (bind _returnvalue_2 (`|CreateWidget` "/Game/UI/WidgetPlayer/End/WBP_End.WBP_End_C" null _mediaplayer))
  (`UserWidget.AddToViewport` _returnvalue_2 0)
  (add `MediaPlayer.OnEndReached` _mediaplayer (delegate `OnEndReached_Event`)))

(event `OnEndReached_Event`
  (`Widget.RemoveFromParent` (stale `self.ReceiveBeginPlay` _returnvalue_2))
  (`GameplayStatics.OpenLevelBySoftObjectPtr` "/Game/Maps/LVL_menu.LVL_menu"))

(fn `UserConstructionScript`)