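; Interactable locked gate that plays a lock-opening animation before the inherited door interaction becomes available.
; Interact runs a key check against WBP_Door_Church and proceeds only when it returns false, firing a one-shot timeline that rolls the lower lock piece.
; When the timeline finishes, the prompt changes to "Открыть" (Open) and a flag lets later interactions that pass the same check call the parent Interact.
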(event `InteractionInterface.Interact`
  (params (InstigatorPawn :type "Pawn Object Reference"))
  (bind _doorlockbottom (`self.DoorLockBottom`))
  (bind (_returnvalue_roll _returnvalue_pitch _returnvalue_yaw) (`KismetMathLibrary.BreakRotator` (`SceneComponent.K2_GetComponentRotation` _doorlockbottom)))
  (bind _output_get (`self.CheckPlayerKey` InstigatorPawn "/Game/UI/InterfaceGame/WBP_Door_Church.WBP_Door_Church_C"))
  (if (not _output_get)
    (`|ExecutionSequence`
      (:`then_0`
        (`/Engine/EditorBlueprintResources/StandardMacros.DoOnce` false
          (:`Completed`
            (bind (_direction _roll) (`Timeline|OpenDoorLock`)
              (:`Update`
                (`SceneComponent.K2_SetWorldRotation` _doorlockbottom (`KismetMathLibrary.MakeRotator` _roll _returnvalue_pitch _returnvalue_yaw) false false))
              (:`Finished`
                (set `self.WidgetText` "Открыть")
                (set `self.bDoorLockOpen` true))))))
      (:`then_1`
        (if (`self.bDoorLockOpen`)
          (`parent.Interact` InstigatorPawn))))))

(fn `GetInteractText`
  (returns (ReturnValue :type Text))
  (return (`self.WidgetText`)))

(fn `UserConstructionScript`
  (`parent.UserConstructionScript`))