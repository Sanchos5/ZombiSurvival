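; BP_OpenGate is an interactable gate that swings open and closed, or plays a closed-door sound when CanBeOpened is false.
; Interact uses Rotation to set the swing direction and IsCreaky to pick the sound.
; IsOpened selects one of two timelines, each driving GateDoor yaw and alternately played or reversed through a FlipFlop.
; A DoOnce ignores further interaction until the timeline finishes, resetting immediately when the gate cannot open.
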(event `InteractionInterface.Interact`
  (params (InstigatorPawn :type "Pawn Object Reference"))
  (if (`self.rotation`)
    (set `self.z` -1.0)
    (else
      (set `self.z` 1.0)))
  (`/Engine/EditorBlueprintResources/StandardMacros.DoOnce` false :!label _label
    (:`Completed`
      (if (`self.CanBeOpened`)
        (if (`self.IsCreaky`)
          (`GameplayStatics.PlaySound2D` "/Game/Sounds/WAV_Door_Creaking.WAV_Door_Creaking" 1.0 1.0 0.0 null null)
          (else
            (`GameplayStatics.PlaySound2D` "/Game/Sounds/WAV_Door_Open.WAV_Door_Open" 1.0 1.0 0.0 null null)))
        (if (`self.IsOpened`)
          (`/Engine/EditorBlueprintResources/StandardMacros.FlipFlop`
            (:`A`
              (bind (_direction _gatedooropenclosetick) (`Timeline|Timeline` :!label _label_2)
                (:`Update`
                  (`SceneComponent.K2_SetRelativeRotation` (`self.GateDoor`) (`KismetMathLibrary.MakeRotator` 0.0 0.0 (* _gatedooropenclosetick (`self.z`))) false false))
                (:`Finished`
                  (goto _label :!via `Reset`))))
            (:`B`
              (goto _label_2 :!via `Reverse`)))
          (else
            (`/Engine/EditorBlueprintResources/StandardMacros.FlipFlop`
              (:`A`
                (bind (_direction_2 _gatedooropenclosetick_2) (`Timeline|GateDoorOpenClose` :!label _label_3)
                  (:`Update`
                    (`SceneComponent.K2_SetRelativeRotation` (`self.GateDoor`) (`KismetMathLibrary.MakeRotator` 0.0 0.0 (* _gatedooropenclosetick_2 (`self.z`))) false false))
                  (:`Finished`
                    (goto _label :!via `Reset`))))
              (:`B`
                (goto _label_3 :!via `Reverse`)))))
        (else
          (`GameplayStatics.PlaySound2D` "/Game/Sounds/WAV_Door_Closed.WAV_Door_Closed" 1.0 1.0 0.0 null null)
          (goto _label :!via `Reset`))))))

(fn `UserConstructionScript`)