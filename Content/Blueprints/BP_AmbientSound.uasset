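; BP_AmbientSound is a box trigger zone that swaps out background audio and changes volumetric fog while BP_Player is inside.
; A counter on the player tracks overlapped boxes, so only the first entry and last exit trigger changes.
; Entry fades out BP_BGSound and exit fades it back in.
; Separate timelines, played on entry and reversed on exit, lerp the height fog's extinction scale between FogOn and FogOff.
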(event `self.Box.OnComponentBeginOverlap`
  (params (OverlappedComponent :type "PrimitiveComponent Object Reference") (OtherActor :type "Actor Object Reference") (OtherComp :type "PrimitiveComponent Object Reference") (OtherBodyIndex :type Integer) (bFromSweep :type Boolean) (SweepResult :type "HitResult Structure (by ref)"))
  (bind _asbp_player (cast `/Game/Characters/Player/BP_Player` OtherActor))
  (bind _overlappedsoundboxes (`/Game/Characters/Player/BP_Player.OverlappedSoundBoxes` _asbp_player))
  (`/Engine/EditorBlueprintResources/StandardMacros.IncrementInt` _overlappedsoundboxes
    (:`  `
      (if (== _overlappedsoundboxes 1)
        (bind _returnvalue (`GameplayStatics.GetActorOfClass` "/Game/Blueprints/BP_BGSound.BP_BGSound_C"))
        (`AudioComponent.FadeOut` (`/Game/Blueprints/BP_BGSound.BGAudioComp` _returnvalue) 2.0 0.0 "Linear")
        (bind _returnvalue_2 (`GameplayStatics.GetActorOfClass` "/Script/Engine.ExponentialHeightFog"))
        (bind (_direction _startfog) (`Timeline|FogBeginOverlap`)
          (:`Update`
            (`ExponentialHeightFogComponent.SetVolumetricFogExtinctionScale` (`ExponentialHeightFog.Component` _returnvalue_2) (`KismetMathLibrary.Lerp` (`self.FogOn`) (`self.FogOff`) _startfog))))))))

(event `self.Box.OnComponentEndOverlap`
  (params (OverlappedComponent :type "PrimitiveComponent Object Reference") (OtherActor :type "Actor Object Reference") (OtherComp :type "PrimitiveComponent Object Reference") (OtherBodyIndex :type Integer))
  (bind _asbp_player (cast `/Game/Characters/Player/BP_Player` OtherActor))
  (bind _overlappedsoundboxes (`/Game/Characters/Player/BP_Player.OverlappedSoundBoxes` _asbp_player))
  (`/Engine/EditorBlueprintResources/StandardMacros.DecrementInt` _overlappedsoundboxes
    (:`  `
      (if (== _overlappedsoundboxes 0)
        (bind _returnvalue (`GameplayStatics.GetActorOfClass` "/Game/Blueprints/BP_BGSound.BP_BGSound_C"))
        (`AudioComponent.FadeIn` (`/Game/Blueprints/BP_BGSound.BGAudioComp` _returnvalue) 2.0 1.0 0.0 "Linear")
        (bind _returnvalue_2 (`GameplayStatics.GetActorOfClass` "/Script/Engine.ExponentialHeightFog"))
        (bind (_direction _startfog) (`Timeline|FogEndOverlap` :!via `Reverse`)
          (:`Update`
            (`ExponentialHeightFogComponent.SetVolumetricFogExtinctionScale` (`ExponentialHeightFog.Component` _returnvalue_2) (`KismetMathLibrary.Lerp` (`self.FogOn`) (`self.FogOff`) _startfog))))))))

(fn `UserConstructionScript`)