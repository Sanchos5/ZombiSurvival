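; Base gun Blueprint that handles shooting, magazine ammo and reloading for the player's weapons.
; Shoot spends a round, plays sound and particles, and damages BP_Zombie via a line trace from above the character along control rotation.
; An empty magazine triggers Reload, which fills it from inventory stacks matching PatronName, with a second pass to top up.
; Both actions update the HUD ammo bar, and reloading also refreshes the inventory UI.
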(event `self.ReceiveBeginPlay`
  (bind _asbp_hud (cast `/Game/UI/BP_HUD` (`PlayerController.GetHUD` (`GameplayStatics.GetPlayerController` 0))))
  (set `self.Player Interface` (`/Game/UI/BP_HUD.PlayerInterface` _asbp_hud)))

(event `self.ReceiveTick`
  (params (DeltaSeconds :type "Float (single-precision)")))

(event `Event_shot`
  (`ActorComponent.Activate` (`self.ParticleSystem`) true))

(event `Shoot`
  ;[1 1 1] Стрелять
  (if (> (`self.DispenserMagazine`) 0)
    (message `/Game/UI/WidgetPlayer/PatronBar/BPI_Patrons.ConsumePatron` (`/Game/UI/InterfaceGame/WBP_InterfacePlayer.WBP_PatronBar` (`self.Player Interface`)))
    (set `self.DispenserMagazine` (- (`self.DispenserMagazine`) 1))
    (`GameplayStatics.PlaySound2D` "/Game/Audio/Explosion02.Explosion02" 1.0 1.0 0.0 null null)
    (`self.ShotLineTrace` (`self.Damage`))
    (`self.Event_shot`)
    (else
      (`self.Reload`)
      (`KismetSystemLibrary.PrintString` "Пустой магазин"))))

(event `Reload`
  ;[1 1 1] Перезарядка
  (`self.ReloadDispenserMagazine`)
  (if (< (`self.Decrement Patrons Int`) (`self.MaxDispenserMagazine`))
    (`self.ReloadDispenserMagazine`))
  (message `/Game/UI/WidgetPlayer/PatronBar/BPI_Patrons.ReloadPatron` (`/Game/UI/InterfaceGame/WBP_InterfacePlayer.WBP_PatronBar` (`self.Player Interface`)) (`self.DispenserMagazine`)))

(fn `DecrementPatrons`
  (params (Array :type "Array of Slot Structure") (Index :type Integer) (IncrementInt :type Integer))
  (bind (_itemid _quantity _itemtype) (break `Slot` (`|GetArrayItem` Array Index)))
  (`KismetArrayLibrary.Array_Set` Array (`local.Index`) (make `Slot` _itemid (- _quantity IncrementInt) _itemtype))
  (`InventoryComponent.UpdateAllInventoryUI` (`self.GetComponentByClass` (`GameplayStatics.GetPlayerCharacter` 0) "/Script/ZombiSurvival.InventoryComponent")))

(fn `ReloadDispenserMagazine`
  (for (_array_element _array_index) (`.MainInventory` (break `AllItem` (`InventoryComponent.AllItems` (`self.GetComponentByClass` (`GameplayStatics.GetPlayerCharacter` 0) "/Script/ZombiSurvival.InventoryComponent"))))
    (bind ((`ItemID` _itemid) (`Quantity` _quantity)) (break `Slot` _array_element))
    (if (and (== (`.RowName` (break `DataTableRowHandle` _itemid)) (`self.PatronName`)) (> _quantity 0))
      (for _ (range 1 (+ _quantity 1))
        (if (>= (`self.DispenserMagazine`) (`self.MaxDispenserMagazine`))
          (break)
          (else
            (`/Engine/EditorBlueprintResources/StandardMacros.IncrementInt` (`self.DispenserMagazine`)
              (:`  `
                (`/Engine/EditorBlueprintResources/StandardMacros.IncrementInt` (`self.Decrement Patrons Int`)))))))
      (`self.DecrementPatrons` (`.MainInventory` (break `AllItem` (`InventoryComponent.AllItems` (`self.GetComponentByClass` (`GameplayStatics.GetPlayerCharacter` 0) "/Script/ZombiSurvival.InventoryComponent")))) _array_index (`self.Decrement Patrons Int`))
      (set `self.Decrement Patrons Int` 0)
      (break))))

(fn `ShotLineTrace`
  (params (damage :type "Float (double-precision)"))
  (bind _returnvalue (`GameplayStatics.GetPlayerCharacter` 0))
  (bind _returnvalue_2 (+ (`self.K2_GetActorLocation` _returnvalue) (0.0 0.0 65.0)))
  (bind _outhit (`KismetSystemLibrary.LineTraceSingle` :`Start` _returnvalue_2 :`End` (+ _returnvalue_2 (* (`KismetMathLibrary.Conv_RotatorToVector` (`Pawn.GetControlRotation` _returnvalue)) 25000.0)) :`TraceChannel` "TraceTypeQuery2" :`bTraceComplex` true :`DrawDebugType` "ForDuration"))
  (bind _asbp_zombie (cast `/Game/Characters/Enemy/BP_Zombie` (`.HitActor` (`GameplayStatics.BreakHitResult` _outhit))))
  (`GameplayStatics.ApplyDamage` _asbp_zombie damage))

(fn `UserConstructionScript`)